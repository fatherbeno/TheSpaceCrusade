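; Player controller for a multiplayer Paper2D game, handling character progression, HUD, loading screen and end-game lobby.
; Loads the character from BP_SaveGameInstance, tracks XP and levels with a growing threshold, updates HUD_SCrusade and saves stats to the slot.
; XP awards and end-zone checks route through GameMode_Paper2D.
; Lobby chat and player-left notices fan out over the GameMode's controller list to each lobby widget, which also shows the player list.
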(event Custom|CreateLoadingScreen
  (bind _returnvalue (UserInterface|CreateWidget "/Game/Widgets/WBP_LoadingScreen.WBP_LoadingScreen_C" self))
  (bind _output_get (Variables|Default|SetLoadingScreen _returnvalue))
  (UserInterface|Viewport|AddtoViewport _output_get 0))

(event Custom|Award%20XP
  (params (Incoming%20Xp :type Float%20%28single-precision%29))
  (Default|AwardXPtoAllPlayers (.AsGame%20Mode%20Paper%202D (Utilities|Casting|CastToGameMode_Paper2D (Game|GetGameMode))) Incoming%20Xp))

(event Custom|SetupInputs
  (bind _self self)
  (Input|SetInputModeGameOnly _self)
  (Variables|Default|SetbShowMouseCursor _self true))

(event Custom|PlayerLeftMessage
  ;[1 1 1] PlayerLeftMessage
  (Networking|SwitchHasAuthority
    (:Authority
      (Variables|Default|SetSenderText "has just left the CRUSADE!")
      (Variables|Default|SetSenderName (Utilities|Struct|BreakBP_Struct_CharacterSave (Variables|Default|GetCharacterInformation)))
      (bind _asgame_mode_paper_2d (Utilities|Casting|CastToGameMode_Paper2D (Game|GetGameMode)))
      (for _array_element (Variables|/Game/Blueprints/GameMode_Paper2D.GameMode_Paper2D_C|GetAllControllers _asgame_mode_paper_2d)
        (bind _aspaper_controller (Utilities|Casting|CastToPaperController _array_element))
        (CallFunction|UpdateChat _aspaper_controller "SERVER" (Utilities|Text|FormatText "\"{SenderName}\" {SenderText}" (Variables|Default|GetSenderName) (Variables|Default|GetSenderText)) "(R=1.000000,G=0.803000,B=0.000000,A=1.000000)")))))

(event Custom|Owning%20Client%20Award%20XP
  (params (Incoming%20XP :type Float%20%28single-precision%29))
  (bind _output_get (Variables|Default|SetCurrentXP (+ Incoming%20XP (Variables|Default|GetCurrentXP))))
  (bind _structout (Utilities|Struct|SetmembersinBP_Struct_CharacterSave (Variables|Default|GetCharacterInformation) _output_get))
  (Variables|Default|SetCharacterInformation _structout)
  (if (>= (/ (+ Incoming%20XP (Variables|Default|GetCurrentXP)) (Variables|Default|GetMaxLevelXP)) 1.0)
    (CallFunction|LevelUp)
    (else
      (Default|UpdatePercentXP (.AsHUD%20SCrusade (Utilities|Casting|CastToHUD_SCrusade (HUD|GetHUD))) (/ (+ Incoming%20XP (Variables|Default|GetCurrentXP)) (Variables|Default|GetMaxLevelXP))))))

(event Custom|LevelUp
  (bind _returnvalue (HUD|GetHUD))
  (bind _ashud_scrusade (Utilities|Casting|CastToHUD_SCrusade _returnvalue))
  (Variables|Default|SetCurrentXP 0.0)
  (Variables|Default|SetMaxLevelXP (+ (Variables|Default|GetMaxLevelXP) (* (Variables|Default|GetMaxLevelXP) 0.15)))
  (bind _output_get (Variables|Default|SetPlayerLevel (+ 1 (Variables|Default|GetPlayerLevel))))
  (Default|UpdatePercentXP _ashud_scrusade 0.0)
  (Default|UpdatePlayerLevel _ashud_scrusade _output_get)
  (bind _structout (Utilities|Struct|SetmembersinBP_Struct_CharacterSave (Variables|Default|GetCharacterInformation) (Variables|Default|GetPlayerLevel) (Variables|Default|GetCurrentXP) (Variables|Default|GetMaxLevelXP)))
  (Variables|Default|SetCharacterInformation _structout))

(event Custom|InitalSetup
  (bind _asbp_save_game_instance (Utilities|Casting|CastToBP_SaveGameInstance (Game|GetGameInstance)))
  (Variables|Default|SetCharacterInformation (Variables|/Game/Blueprints/SaveData/BP_SaveGameInstance.BP_SaveGameInstance_C|GetLoadedCharacter _asbp_save_game_instance))
  (Variables|Default|SetOldConnectedPlayers (Variables|/Game/Blueprints/SaveData/BP_SaveGameInstance.BP_SaveGameInstance_C|GetOldConnectedPlayers _asbp_save_game_instance))
  (Default|EveryoneUpdates (.AsGame%20Mode%20Paper%202D (Utilities|Casting|CastToGameMode_Paper2D (Game|GetGameMode)))))

(event Custom|ApplyDynamicMaterial
  (bind _aspaper_2d_character (Utilities|Casting|CastToPaper2D_Character (Pawn|GetControlledPawn)))
  (Default|CreateDynamicMaterial _aspaper_2d_character))

(event Custom|CheckPlayerIsFinished
  (params (bPlayerEnteredEndZone? :type Boolean))
  (Default|AreAllPlayersFinished? (.AsGame%20Mode%20Paper%202D (Utilities|Casting|CastToGameMode_Paper2D (Game|GetGameMode))) self bPlayerEnteredEndZone?))

(event Custom|SetupLobbyMenu
  (params (ServerName :type Text))
  ;[1 1 1] DisplayLobbyMenu
  (Utilities|IsValid (Variables|Default|GetGameEndWidgetReference)
    (:Is%20Not%20Valid
      (bind _returnvalue (UserInterface|CreateWidget "/Game/Widgets/WBP_EndGameLobby.WBP_EndGameLobby_C" 0 ServerName))
      (bind _output_get (Variables|Default|SetGameEndWidgetReference _returnvalue))
      (UserInterface|Viewport|AddtoViewport _output_get 0))))

(event Custom|DeleteLoadingScreen
  (bind _loadingscreen (Variables|Default|GetLoadingScreen))
  (Utilities|IsValid _loadingscreen
    (:Is%20Valid
      (Widget|RemovefromParent _loadingscreen))))

(event Custom|GetChatMessage
  (params (TextToSend :type Text))
  (bind _characterinformation (Variables|Default|GetCharacterInformation))
  (bind (_name _highlightcolour) (Utilities|Struct|BreakBP_Struct_CharacterSave _characterinformation))
  ;[1 1 1] Processes Incoming Chat, Updates Chat
  (Variables|Default|SetSenderText TextToSend)
  (Variables|Default|SetSenderName _name)
  (Variables|Default|SetSenderColour _highlightcolour)
  (bind _asgame_mode_paper_2d (Utilities|Casting|CastToGameMode_Paper2D (Game|GetGameMode)))
  (for _array_element (Variables|/Game/Blueprints/GameMode_Paper2D.GameMode_Paper2D_C|GetAllControllers _asgame_mode_paper_2d)
    (bind _aspaper_controller (Utilities|Casting|CastToPaperController _array_element))
    (CallFunction|UpdateChat _aspaper_controller (Variables|Default|GetSenderName) (Variables|Default|GetSenderText) (Variables|Default|GetSenderColour))))

(event Custom|SaveUpdatedPlayerStats
  (bind _asbp_save_game_instance (Utilities|Casting|CastToBP_SaveGameInstance (Game|GetGameInstance)))
  (bind _structout (Utilities|Struct|SetmembersinBP_Struct_CharacterSave (Utilities|Array|Get(acopy) (Variables|/Game/Blueprints/SaveData/BP_PlayerSaveData.BP_PlayerSaveData_C|GetCharacters (Variables|/Game/Blueprints/SaveData/BP_SaveGameInstance.BP_SaveGameInstance_C|GetSaveGameData _asbp_save_game_instance)) (Variables|/Game/Blueprints/SaveData/BP_SaveGameInstance.BP_SaveGameInstance_C|GetLoadedCharacterIndex _asbp_save_game_instance)) (Variables|Default|GetPlayerLevel) (Variables|Default|GetCurrentXP) (Variables|Default|GetMaxLevelXP)))
  (Variables|Default|SetCharacterInformation _structout)
  (SaveGame|SaveGametoSlot (Variables|/Game/Blueprints/SaveData/BP_SaveGameInstance.BP_SaveGameInstance_C|GetSaveGameData _asbp_save_game_instance) (Variables|/Game/Blueprints/SaveData/BP_SaveGameInstance.BP_SaveGameInstance_C|GetSaveGameSlot _asbp_save_game_instance)))

(event Custom|SetupHUD
  (bind _characterinformation (Variables|Default|GetCharacterInformation))
  (bind (_characterlevel _currentexperience _maxlevelxp) (Utilities|Struct|BreakBP_Struct_CharacterSave _characterinformation))
  (Variables|Default|SetPlayerLevel _characterlevel)
  (Variables|Default|SetCurrentXP _currentexperience)
  (Variables|Default|SetMaxLevelXP (select (== _maxlevelxp 0.0) 1e+02 _maxlevelxp))
  (bind _ashud_scrusade (Utilities|Casting|CastToHUD_SCrusade (HUD|GetHUD)))
  (Default|CreateHUD _ashud_scrusade self)
  (Default|UpdatePercentXP _ashud_scrusade (/ (Variables|Default|GetCurrentXP) (Variables|Default|GetMaxLevelXP)))
  (Default|UpdatePlayerLevel _ashud_scrusade (Variables|Default|GetPlayerLevel))
  (bind _asgame_mode_paper_2d (Utilities|Casting|CastToGameMode_Paper2D (Game|GetGameMode)))
  (EventDispatchers|BindEventtoXPDispatcher _asgame_mode_paper_2d (delegate Custom|Award%20XP)))

(event Custom|UpdateChat
  (params (Sender :type Text) (InputText :type Text) (SenderColour :type Linear%20Color%20Structure))
  ;[1 1 1] Update Chat
  (Default|UpdateChatWindow (Variables|Default|GetGameEndWidgetReference) Sender InputText SenderColour))

(event Custom|AddPlayerInformation
  (params (Connected%20Player%20Information :type BP%20Struct%20Character%20Save%20Structure))
  (bind _gameendwidgetreference (Variables|Default|GetGameEndWidgetReference))
  ;[1 1 1] Update Player List Window
  (Utilities|IsValid _gameendwidgetreference
    (:Is%20Valid
      (Default|ClearPlayerList _gameendwidgetreference)
      (Default|UpdatePlayerWindow _gameendwidgetreference Connected%20Player%20Information))))

(fn ConstructionScript)