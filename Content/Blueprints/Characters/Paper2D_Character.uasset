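; Player Paper2D character with eight-direction walk and idle flipbooks, a cursor-aimed sword, a pause menu and a saved highlight colour.
; Each locally controlled Tick picks a flipbook from input and velocity, then passes it and the cursor-facing spring arm rotation to ServerUpdateRotations.
; Sword input, throttled by a timer, spawns S_Sword attached at an arrow through ServerSwordAttack.
; BeginPlay applies the GameInstance colour through a dynamic material after a delay.
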(event Custom|ServerSwordAttack
  (params (yRotation :type Float%20%28single-precision%29) (zRotation :type Float%20%28single-precision%29) (Spawn%20Location :type Vector) (Attach%20Point :type Scene%20Component%20Object%20Reference))
  ;[1 1 1] PlayerAttacking
  (Utilities|SwordAttack (Math|Rotator|MakeRotator 0.0 yRotation zRotation) Spawn%20Location Attach%20Point))

(event Custom|ResetSwing
  ;[1 1 1] PlayerAttacking
  (Variables|Character|SetisSwinging? false))

(event Custom|PauseUnpauseGame
  (bind _returnvalue (Game|GetPlayerController 0))
  (bind _gameinstancereference (Variables|DisplayCharacter|GetGameInstanceReference))
  ;[1 1 1] Pause Menu
  (bind _output_get (Variables|/Game/Blueprints/SaveData/BP_SaveGameInstance.BP_SaveGameInstance_C|SetbIsGamePaused _gameinstancereference (not (Variables|/Game/Blueprints/SaveData/BP_SaveGameInstance.BP_SaveGameInstance_C|GetbIsGamePaused _gameinstancereference))))
  (Game|SetGamePaused _output_get)
  (if _output_get
    (bind _returnvalue_2 (UserInterface|CreateWidget "/Game/Widgets/WBP_PauseMenu.WBP_PauseMenu_C"))
    (bind _output_get_2 (Variables|Default|SetPauseMenuReference _returnvalue_2))
    (UserInterface|Viewport|AddtoViewport _output_get_2 0)
    (EventDispatchers|BindEventtoPauseUnpauseEventDispatcher _output_get_2 (delegate Custom|PauseUnpauseGame))
    (Input|SetInputModeGameandUI _returnvalue (Variables|Default|GetPauseMenuReference) "DoNotLock" false)
    (Variables|/Script/Engine.PlayerController|SetbShowMouseCursor _returnvalue true)
    (elif (Utilities|IsValid (Variables|Default|GetPauseMenuReference))
      (Widget|RemovefromParent (Variables|Default|GetPauseMenuReference))
      (Variables|Default|SetPauseMenuReference 0)
      (Input|SetInputModeGameOnly _returnvalue)
      (Variables|/Script/Engine.PlayerController|SetbShowMouseCursor _returnvalue true))))

(event Custom|serverUpdateRotations
  (params (New%20Flipbook :type Paper%20Flipbook%20Object%20Reference) (Spring%20arm :type Scene%20Component%20Object%20Reference) (Target :type Paper%20Flipbook%20Component%20Object%20Reference) (Spring%20arm%20rotation :type Rotator))
  ;[1 1 1] Weapon Rotation and set the character's walking animation
  (Transformation|SetWorldRotation Spring%20arm Spring%20arm%20rotation false false)
  (Sprite|SetFlipbook Target New%20Flipbook))

(event EventBeginPlay
  ;[1 1 1] CharacterCustomizedColor
  (Utilities|FlowControl|Delay 2.0)
  (bind _ashud_scrusade (Utilities|Casting|CastToHUD_SCrusade (HUD|GetHUD (Game|GetPlayerController 0))))
  (Variables|Default|SetPlayerHUD _ashud_scrusade)
  (bind _returnvalue (Rendering|Material|CreateDynamicMaterialInstance (Variables|Default|GetSprite) 0 "/Game/Materials/Int_Cosmestic_Color.Int_Cosmestic_Color" "None" :!class /Script/Engine.PrimitiveComponent))
  (Variables|DisplayCharacter|SetDynamicColourInstance _returnvalue)
  (bind _asbp_save_game_instance (Utilities|Casting|CastToBP_SaveGameInstance (Game|GetGameInstance)))
  (bind _output_get (Variables|DisplayCharacter|SetGameInstanceReference _asbp_save_game_instance))
  (Rendering|Material|SetVectorParameterValue (Variables|DisplayCharacter|GetDynamicColourInstance) "Base Colour" (.highlightcolour (Variables|/Game/Blueprints/SaveData/BP_SaveGameInstance.BP_SaveGameInstance_C|GetLoadedCharacter _output_get)) :!class /Script/Engine.MaterialInstanceDynamic))

(event EventTick
  (params (DeltaSeconds :type Float%20%28single-precision%29))
  ;[1 1 1] Weapon Rotation and set the character's walking animation
  (if (Pawn|IsLocallyControlled)
    (bind (_target _new_flipbook) (CallFunction|SetDirection))
    (CallFunction|ServerUpdateRotations _new_flipbook (Variables|Default|GetSpringArm1) _target (Math|Rotator|MakeRotator 9e+01 (.roll (Transformation|GetActorRotation)) (+ (.yaw (Math|Rotator|FindLookatRotation (Transformation|GetActorLocation) (.Location (Collision|BreakHitResult (.HitResult (Game|Player|GetHitResultUnderCursorbyChannel (Game|GetPlayerController 0) "TraceTypeQuery1" true)))))) -1.8e+02)))))

(event Input|ActionEvents|InputActionSwordAttack
  (params (Key :type Key%20Structure :default "None"))
  ;[1 1 1] PlayerAttacking
  (:Pressed
    (if (not (Variables|Character|GetisSwinging?))
      (Variables|Character|SetisSwinging? true)
      (Utilities|Time|SetTimerbyEvent (delegate Custom|ResetSwing) 0.5)
      (CallFunction|ServerSwordAttack self (.pitch (Transformation|GetActorRotation)) (+ (.yaw (Math|Rotator|FindLookatRotation (Transformation|GetActorLocation) (.Location (Collision|BreakHitResult (.HitResult (Game|Player|GetHitResultUnderCursorbyChannel (Game|GetPlayerController 0) "TraceTypeQuery1" true)))))) -1.8e+02) (Transformation|GetWorldLocation (Variables|Default|GetArrow1)) (Variables|Default|GetArrow1)))))

(event Input|ActionEvents|InputActionPause
  (params (Key :type Key%20Structure :default "None"))
  (bind _returnvalue (Game|GetPlayerController 0))
  (bind _gameinstancereference (Variables|DisplayCharacter|GetGameInstanceReference))
  ;[1 1 1] Pause Menu
  (:Pressed
    (bind _output_get (Variables|/Game/Blueprints/SaveData/BP_SaveGameInstance.BP_SaveGameInstance_C|SetbIsGamePaused _gameinstancereference (not (Variables|/Game/Blueprints/SaveData/BP_SaveGameInstance.BP_SaveGameInstance_C|GetbIsGamePaused _gameinstancereference))))
    (Game|SetGamePaused _output_get)
    (if _output_get
      (bind _returnvalue_2 (UserInterface|CreateWidget "/Game/Widgets/WBP_PauseMenu.WBP_PauseMenu_C"))
      (bind _output_get_2 (Variables|Default|SetPauseMenuReference _returnvalue_2))
      (UserInterface|Viewport|AddtoViewport _output_get_2 0)
      (EventDispatchers|BindEventtoPauseUnpauseEventDispatcher _output_get_2 (delegate Custom|PauseUnpauseGame))
      (Input|SetInputModeGameandUI _returnvalue (Variables|Default|GetPauseMenuReference) "DoNotLock" false)
      (Variables|/Script/Engine.PlayerController|SetbShowMouseCursor _returnvalue true)
      (elif (Utilities|IsValid (Variables|Default|GetPauseMenuReference))
        (Widget|RemovefromParent (Variables|Default|GetPauseMenuReference))
        (Variables|Default|SetPauseMenuReference 0)
        (Input|SetInputModeGameOnly _returnvalue)
        (Variables|/Script/Engine.PlayerController|SetbShowMouseCursor _returnvalue true)))))

(event Input|AxisEvents|InputAxisXAxis
  (params (AxisValue :type Float%20%28single-precision%29))
  ;[1 1 1] Player's Movement
  (Pawn|Input|AddMovementInput (* (Math|Vector|Normalize (+ (Math|Vector|MakeVector 0.0 1.0 0.0) (Math|Vector|MakeVector 1.0 0.0 0.0))) "0,-1.000000, 0") AxisValue true))

(event Input|AxisEvents|InputAxisYAxis
  (params (AxisValue :type Float%20%28single-precision%29))
  ;[1 1 1] Player's Movement
)

(event Input|TouchEvents|InputTouch
  (params (Location :type Vector) (FingerIndex :type ETouchIndex%20Enum))
  ;[1 1 1] Player's Movement
  (:Pressed
    (Variables|Default|SetLast_Touched_Location Location))
  (:Moved
    (Pawn|Input|AddMovementInput (- Location (Variables|Default|GetLast_Touched_Location)) (Variables|Default|GetTouch_Strength) true)))

(fn ConstructionScript
  (Transformation|SetWorldRotation (Variables|Default|GetSprite) (Math|Rotator|MakeRotator (.pitch (Transformation|GetWorldRotation (Variables|Camera|GetSpringArm))) 0.0 -9e+01) false false))

(fn SetDirection
  ;[1 1 1] Idle Animation
  (if (or (!= (Input|AxisValues|GetXAxis) 0.0) (!= (Input|AxisValues|GetYAxis) 0.0))
    (Variables|Animation|SetDirection (select (and (> (Input|AxisValues|GetXAxis) 0.0) (> (Input|AxisValues|GetYAxis) 0.0)) "NewEnumerator4" (select (and (< (Input|AxisValues|GetXAxis) 0.0) (< (Input|AxisValues|GetYAxis) 0.0)) "NewEnumerator7" (select (and (> (Input|AxisValues|GetXAxis) 0.0) (< (Input|AxisValues|GetYAxis) 0.0)) "NewEnumerator6" (select (and (< (Input|AxisValues|GetXAxis) 0.0) (> (Input|AxisValues|GetYAxis) 0.0)) "NewEnumerator5" (select (> (Input|AxisValues|GetYAxis) 0.0) "NewEnumerator0" (select (< (Input|AxisValues|GetYAxis) 0.0) "NewEnumerator1" (select (> (Input|AxisValues|GetXAxis) 0.0) "NewEnumerator2" "NewEnumerator3"))))))))
    (if true
      (return (Variables|Default|GetSprite) (select (> (Math|Vector|VectorLength (Transformation|GetVelocity)) 0.0) (Utilities|Select :Index (Variables|Animation|GetDirection) :NewEnumerator0 "/Game/Sprites/CharacterUpdate/FB_SpriteWalkingUp.FB_SpriteWalkingUp" :NewEnumerator1 "/Game/Sprites/CharacterUpdate/FB_SpriteWalkingDown.FB_SpriteWalkingDown" :NewEnumerator2 "/Game/Sprites/CharacterUpdate/FB_SpriteWalkingRight.FB_SpriteWalkingRight" :NewEnumerator3 "/Game/Sprites/CharacterUpdate/FB_SpriteWalkingLeft.FB_SpriteWalkingLeft" :NewEnumerator4 "/Game/Sprites/CharacterUpdate/FB_SpriteWalkingNorthEast.FB_SpriteWalkingNorthEast" :NewEnumerator5 "/Game/Sprites/CharacterUpdate/FB_SpriteWalkingNWest.FB_SpriteWalkingNWest" :NewEnumerator6 "/Game/Sprites/CharacterUpdate/FB_WalkingSouthEast.FB_WalkingSouthEast" :NewEnumerator7 "/Game/Sprites/CharacterUpdate/FB_SpriteWalkingSouthWest.FB_SpriteWalkingSouthWest") (Utilities|Select :Index (Variables|Animation|GetDirection) :NewEnumerator0 "/Game/Sprites/CharacterUpdate/BaseIdle/IdleUp.IdleUp" :NewEnumerator1 "/Game/Sprites/CharacterUpdate/BaseIdle/IdleDown.IdleDown" :NewEnumerator2 "/Game/Sprites/CharacterUpdate/BaseIdle/IdleRight.IdleRight" :NewEnumerator3 "/Game/Sprites/CharacterUpdate/BaseIdle/IdleLeft.IdleLeft" :NewEnumerator4 "/Game/Sprites/CharacterUpdate/BaseIdle/IdleNE.IdleNE" :NewEnumerator5 "/Game/Sprites/CharacterUpdate/BaseIdle/IdleNW.IdleNW" :NewEnumerator6 "/Game/Sprites/CharacterUpdate/BaseIdle/IdleSE.IdleSE" :NewEnumerator7 "/Game/Sprites/CharacterUpdate/BaseIdle/IdleSW.IdleSW")))
      (else
        _)))
  (return (Variables|Default|GetSprite) (select (> (Math|Vector|VectorLength (Transformation|GetVelocity)) 0.0) (Utilities|Select :Index (Variables|Animation|GetDirection) :NewEnumerator0 "/Game/Sprites/CharacterUpdate/FB_SpriteWalkingUp.FB_SpriteWalkingUp" :NewEnumerator1 "/Game/Sprites/CharacterUpdate/FB_SpriteWalkingDown.FB_SpriteWalkingDown" :NewEnumerator2 "/Game/Sprites/CharacterUpdate/FB_SpriteWalkingRight.FB_SpriteWalkingRight" :NewEnumerator3 "/Game/Sprites/CharacterUpdate/FB_SpriteWalkingLeft.FB_SpriteWalkingLeft" :NewEnumerator4 "/Game/Sprites/CharacterUpdate/FB_SpriteWalkingNorthEast.FB_SpriteWalkingNorthEast" :NewEnumerator5 "/Game/Sprites/CharacterUpdate/FB_SpriteWalkingNWest.FB_SpriteWalkingNWest" :NewEnumerator6 "/Game/Sprites/CharacterUpdate/FB_WalkingSouthEast.FB_WalkingSouthEast" :NewEnumerator7 "/Game/Sprites/CharacterUpdate/FB_SpriteWalkingSouthWest.FB_SpriteWalkingSouthWest") (Utilities|Select :Index (Variables|Animation|GetDirection) :NewEnumerator0 "/Game/Sprites/CharacterUpdate/BaseIdle/IdleUp.IdleUp" :NewEnumerator1 "/Game/Sprites/CharacterUpdate/BaseIdle/IdleDown.IdleDown" :NewEnumerator2 "/Game/Sprites/CharacterUpdate/BaseIdle/IdleRight.IdleRight" :NewEnumerator3 "/Game/Sprites/CharacterUpdate/BaseIdle/IdleLeft.IdleLeft" :NewEnumerator4 "/Game/Sprites/CharacterUpdate/BaseIdle/IdleNE.IdleNE" :NewEnumerator5 "/Game/Sprites/CharacterUpdate/BaseIdle/IdleNW.IdleNW" :NewEnumerator6 "/Game/Sprites/CharacterUpdate/BaseIdle/IdleSE.IdleSE" :NewEnumerator7 "/Game/Sprites/CharacterUpdate/BaseIdle/IdleSW.IdleSW"))))