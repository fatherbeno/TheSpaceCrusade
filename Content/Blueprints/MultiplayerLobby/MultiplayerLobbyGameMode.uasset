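; Game mode for the multiplayer lobby, managing joining players, ready checks, kicking and match launch.
; On server login it stores each controller, sets up its lobby menu with the saved server name, then runs EveryoneUpdate.
; That update gathers character information, pushes the roster and count to every controller, and sets CanWeStart from ready flags.
; Launch server-travels to ProGenTest, while kick-list and colour-change events are empty stubs.
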(event Custom|ChangeCharacterColour
  (params (PlayerController :type Player%20Controller%20Object%20Reference) (CharacterColour :type Linear%20Color%20Structure) (ChangedStatus :type Boolean)))

(event Custom|EveryoneUpdate
  ;[1 1 1] Everyone Update
  (bind _output_get (Variables|ServerSettings|SetCurrentPlayers (Utilities|Array|Length (Variables|ServerSettings|GetAllPlayerControllers))))
  (if (> _output_get 0)
    (Utilities|Array|Clear (Variables|ServerSettings|GetConnectedPlayers))
    (for _array_element (Variables|ServerSettings|GetAllPlayerControllers)
      (bind _asmultiplayer_lobby_player_controller (Utilities|Casting|CastToMultiplayerLobbyPlayerController _array_element))
      (Utilities|Array|Add (Variables|ServerSettings|GetConnectedPlayers) (Variables|/Game/Blueprints/MultiplayerLobby/MultiplayerLobbyPlayerController.MultiplayerLobbyPlayerController_C|GetCharacterInformation _asmultiplayer_lobby_player_controller))
      (Default|UpdateNumberOfPlayers _asmultiplayer_lobby_player_controller (Variables|ServerSettings|GetCurrentPlayers)))
    (for _array_element_2 (Variables|ServerSettings|GetAllPlayerControllers)
      (bind _asmultiplayer_lobby_player_controller_2 (Utilities|Casting|CastToMultiplayerLobbyPlayerController _array_element_2))
      (Default|AddPlayerInformation _asmultiplayer_lobby_player_controller_2 (Variables|ServerSettings|GetConnectedPlayers))
      (CallFunction|AddtoKickList))
    (bind _array_element_3 (Utilities|Array|ForEachLoopwithBreak (Variables|ServerSettings|GetConnectedPlayers))
      (:LoopBody
        (if (Utilities|Struct|BreakBP_Struct_CharacterSave _array_element_3)
          (Variables|ServerSettings|SetbCanWeStart? true)
          (else
            (Variables|ServerSettings|SetbCanWeStart? false)
            (CallFunction|CannotStartGame)))))))

(event Custom|LaunchTheGame
  (bind _returnvalue (Game|GetPlayerController 0))
  (Input|SetInputModeGameOnly _returnvalue)
  (Variables|/Script/Engine.PlayerController|SetbShowMouseCursor _returnvalue true)
  (Development|ExecuteConsoleCommand "servertravel /Game/Levels/ProGenTest" _returnvalue))

(event Custom|AddToKickList)

(event Custom|CannotStartGame
  ;[1 1 1] Everyone Update
  (Utilities|Array|ForEachLoopwithBreak (Variables|ServerSettings|GetConnectedPlayers)) ; enters at Break
)

(event Custom|YouHaveBeenKicked
  (params (PlayerID :type Integer))
  ;[1 1 1] Kick the selected player
  (Default|Kicked (.AsMultiplayer%20Lobby%20Player%20Controller (Utilities|Casting|CastToMultiplayerLobbyPlayerController (Utilities|Array|Get(acopy) (Variables|ServerSettings|GetAllPlayerControllers) PlayerID)))))

(event EventPostLogin
  (params (NewPlayer :type Player%20Controller%20Object%20Reference))
  ;[1 1 1] Initial Setup after Player Logs In
  (Networking|SwitchHasAuthority
    (:Authority
      (Utilities|Array|Add (Variables|ServerSettings|GetAllPlayerControllers) NewPlayer)
      (bind _asbp_save_game_instance (Utilities|Casting|CastToBP_SaveGameInstance (Game|GetGameInstance)))
      (Variables|ServerSettings|SetServerName (Variables|/Game/Blueprints/SaveData/BP_SaveGameInstance.BP_SaveGameInstance_C|GetServerName _asbp_save_game_instance))
      (bind _asmultiplayer_lobby_player_controller (Utilities|Casting|CastToMultiplayerLobbyPlayerController NewPlayer))
      (Default|InitialSetup _asmultiplayer_lobby_player_controller)
      (Default|SetupLobbyMenu _asmultiplayer_lobby_player_controller (Variables|ServerSettings|GetServerName))
      (CallFunction|EveryoneUpdate))))

(fn ConstructionScript)