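; DoorTry is an experimental Paper2D door Blueprint that picks a flipbook animation for its render component.
; Its Dooranim function branches on the DoorOpen flag and feeds enum-driven selects into the new flipbook.
; The outer select condition is fixed false, so both paths resolve to the open-idle flipbook.
; The event graph and construction script are empty, and nothing here calls Dooranim.
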(event EventBeginPlay)

(event Collision|EventActorBeginOverlap
  (params (OtherActor :type Actor%20Object%20Reference)))

(event EventTick
  (params (DeltaSeconds :type Float%20%28single-precision%29)))

(fn ConstructionScript)

(fn Dooranim
  (bind _endoor (Variables|Default|GetEnDoor))
  (bind _returnvalue (Utilities|Select :Index _endoor :NewEnumerator0 "/Game/Sprites/TileMap/SpaceShip_Tilemap/SpaceShip_Door/DoorOpen.DoorOpen" :NewEnumerator1 "/Game/Sprites/TileMap/SpaceShip_Tilemap/SpaceShip_Door/DoorClose.DoorClose"))
  (bind _returnvalue_2 (Utilities|Select :Index _endoor :NewEnumerator0 "/Game/Sprites/TileMap/SpaceShip_Tilemap/SpaceShip_Door/DoorIdleOpen.DoorIdleOpen" :NewEnumerator1 "/Game/Sprites/TileMap/SpaceShip_Tilemap/SpaceShip_Door/DoorIdleOpen.DoorIdleOpen"))
  (bind _returnvalue_3 (select false _returnvalue _returnvalue_2))
  (if (Variables|Default|GetDoorOpen)
    (return (Variables|Default|GetRenderComponent) _returnvalue_3)
    (else
      (Variables|Default|SetDoorOpen false)
      (return (Variables|Default|GetRenderComponent) _returnvalue_3))))