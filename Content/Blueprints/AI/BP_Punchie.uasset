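; BP_Punchie is a damageable AI character with directional Paper2D flipbook animation that awards XP on death.
; Damage lowers Health and stores the instigator; at zero it reports XP to the game mode, disables capsule collision and destroys itself after a delay.
; A looping quarter-second timer picks the facing from the dominant velocity axis.
; UpdateAnimation changes flipbooks only on a new direction while moving, leaving its idle branch effectively unused.
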(event Custom|Custom%20Tick%20Quater-Second
  (bind _charactermovement (Variables|Character|GetCharacterMovement))
  (bind _returnvalue (Pawn|Components|CharacterMovement|GetLastUpdateVelocity _charactermovement))
  (bind _returnvalue_2 (Math|Float|Absolute(Float) (.x _returnvalue)))
  (bind _returnvalue_3 (Math|Float|Absolute(Float) (.y _returnvalue)))
  (if (not (== _returnvalue_2 _returnvalue_3))
    (if (> _returnvalue_2 _returnvalue_3)
      (if (> (.x _returnvalue) 0.0)
        (bind (_target _new_flipbook) (CallFunction|UpdateAnimation "NewEnumerator1"))
        (Sprite|SetFlipbook _target _new_flipbook)
        (else
          (bind (_target_2 _new_flipbook_2) (CallFunction|UpdateAnimation "NewEnumerator0"))
          (Sprite|SetFlipbook _target_2 _new_flipbook_2)))
      (elif (> (.y _returnvalue) 0.0)
        (bind (_target_3 _new_flipbook_3) (CallFunction|UpdateAnimation "NewEnumerator2"))
        (Sprite|SetFlipbook _target_3 _new_flipbook_3)
        (else
          (bind (_target_4 _new_flipbook_4) (CallFunction|UpdateAnimation "NewEnumerator3"))
          (Sprite|SetFlipbook _target_4 _new_flipbook_4))))))

(event Custom|GiveXp
  (Class|INTPlayer|AddXP(Message) (Game|GetGameMode) (Variables|Default|GetXP)))

(event EventBeginPlay
  (Utilities|Time|SetTimerbyEvent (delegate Custom|Custom%20Tick%20Quater-Second) 0.25 true))

(event Game|Damage|EventAnyDamage
  (params (Damage :type Float%20%28single-precision%29) (DamageType :type Damage%20Type%20Object%20Reference) (InstigatedBy :type Controller%20Object%20Reference) (DamageCauser :type Actor%20Object%20Reference))
  (Variables|Default|SetPlayer InstigatedBy)
  (Variables|Default|SetHealth (- (Variables|Default|GetHealth) Damage))
  (if (<= (Variables|Default|GetHealth) 0.0)
    (CallFunction|GiveXP)
    (Collision|SetCollisionEnabled (Variables|Collision|GetCapsuleComponent) "NoCollision")
    (Utilities|FlowControl|Delay 5.0)
    (Actor|DestroyActor)))

(fn ConstructionScript)

(fn UpdateAnimation
  (params (New_Direction :type En_SetDirection_Enemy%20Enum :default "NewEnumerator0"))
  (bind _returnvalue (Transformation|GetVelocity))
  ;[1 1 1] Idle
  (if (not (== New_Direction (Variables|Default|GetSetAnimation)))
    (if (or (!= 0.0 (.x _returnvalue)) (!= 0.0 (.y _returnvalue)))
      (Variables|Default|SetSetAnimation New_Direction)
      (if true
        (return (Variables|Default|GetSprite) (select (> (Math|Vector|VectorLength (Transformation|GetVelocity)) 0.0) (Utilities|Select :Index (Variables|Default|GetSetAnimation) :NewEnumerator0 "/Game/Sprites/Enemy/UP/P_WalkingUp.P_WalkingUp" :NewEnumerator1 "/Game/Sprites/Enemy/Down/P_WalkingDown.P_WalkingDown" :NewEnumerator2 "/Game/Sprites/Enemy/Left/P_WalkingLeft.P_WalkingLeft" :NewEnumerator3 "/Game/Sprites/Enemy/Right/P_WalkingRight.P_WalkingRight" :NewEnumerator4 0 :NewEnumerator5 0 :NewEnumerator6 0) (Utilities|Select :Index (Variables|Default|GetSetAnimation) :NewEnumerator0 "/Game/Sprites/Enemy/UP/P_IdleUp.P_IdleUp" :NewEnumerator1 "/Game/Sprites/Enemy/Down/P_IdleDown.P_IdleDown" :NewEnumerator2 "/Game/Sprites/Enemy/Left/P_IdleLeft.P_IdleLeft" :NewEnumerator3 "/Game/Sprites/Enemy/Right/P_IdleRight.P_IdleRight" :NewEnumerator4 0 :NewEnumerator5 0 :NewEnumerator6 0)))
        (else
          (return (Variables|Default|GetSprite) (select (> (Math|Vector|VectorLength (Transformation|GetVelocity)) 0.0) (Utilities|Select :Index (Variables|Default|GetSetAnimation) :NewEnumerator0 "/Game/Sprites/Enemy/UP/P_WalkingUp.P_WalkingUp" :NewEnumerator1 "/Game/Sprites/Enemy/Down/P_WalkingDown.P_WalkingDown" :NewEnumerator2 "/Game/Sprites/Enemy/Left/P_WalkingLeft.P_WalkingLeft" :NewEnumerator3 "/Game/Sprites/Enemy/Right/P_WalkingRight.P_WalkingRight" :NewEnumerator4 0 :NewEnumerator5 0 :NewEnumerator6 0) (Utilities|Select :Index (Variables|Default|GetSetAnimation) :NewEnumerator0 "/Game/Sprites/Enemy/UP/P_IdleUp.P_IdleUp" :NewEnumerator1 "/Game/Sprites/Enemy/Down/P_IdleDown.P_IdleDown" :NewEnumerator2 "/Game/Sprites/Enemy/Left/P_IdleLeft.P_IdleLeft" :NewEnumerator3 "/Game/Sprites/Enemy/Right/P_IdleRight.P_IdleRight" :NewEnumerator4 0 :NewEnumerator5 0 :NewEnumerator6 0))))))))