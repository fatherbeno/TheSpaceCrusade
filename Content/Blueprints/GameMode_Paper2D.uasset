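; Multiplayer game mode for a Paper2D game, managing player joins, XP awards, damage, respawns and match end.
; PostLogin spawns and possesses a character, then refreshes every controller's player list, HUD, inputs and materials.
; Any player newly entering the end zone ends the game for all, opening lobby menus and saving stats.
; Respawn restores the "check" save location or reopens the level; hurt never triggers it because DamageAnimation always returns false.
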(event Custom|EveryoneUpdates
  (Utilities|Array|Clear (Variables|Default|GetConnectedPlayers))
  (for _array_element (Variables|Default|GetAllControllers)
    (bind _aspaper_controller (Utilities|Casting|CastToPaperController _array_element))
    (Utilities|Array|Add (Variables|Default|GetConnectedPlayers) (Variables|/Game/Blueprints/Characters/PaperController.PaperController_C|GetCharacterInformation _aspaper_controller))
    (Default|SetupHUD _aspaper_controller)
    (Default|SetupInputs _aspaper_controller)
    (Variables|Default|SetOldConnectedPlayers (Variables|/Game/Blueprints/Characters/PaperController.PaperController_C|GetOldConnectedPlayers _aspaper_controller)))
  (if (== (Utilities|Array|Length (Variables|Default|GetConnectedPlayers)) (Utilities|Array|Length (Variables|Default|GetOldConnectedPlayers)))
    _
    (else
      (Utilities|FlowControl|RetriggerableDelay 5.0)))
  (for _array_element_2 (Variables|Default|GetAllControllers)
    (bind _aspaper_controller_2 (Utilities|Casting|CastToPaperController _array_element_2))
    (Default|ApplyDynamicMaterial _aspaper_controller_2)))

(event Custom|PlayerHurt
  (params (PlayerController :type Paper%20Controller%20Object%20Reference))
  (bind _aspaper_2d_character (Utilities|Casting|CastToPaper2D_Character (Pawn|GetControlledPawn PlayerController)))
  (Default|PlaySound _aspaper_2d_character)
  (bind _healthcheck (CallFunction|DamageAnimation _aspaper_2d_character))
  (Utilities|FlowControl|Delay 0.15)
  (Transformation|SetActorRelativeScale3D _aspaper_2d_character "0.800000,1.000000,0.800000")
  (if _healthcheck
    (Utilities|Respawn PlayerController _aspaper_2d_character)))

(event Custom|Multicast%20Award%20XP
  (params (Incoming%20XP :type Float%20%28single-precision%29))
  (Default|CallXPDispatcher Incoming%20XP))

(event Custom|GameIsFinished
  (Utilities|Array|Clear (Variables|Default|GetConnectedPlayers))
  (for _array_element (Variables|Default|GetAllControllers)
    (bind _aspaper_controller (Utilities|Casting|CastToPaperController _array_element))
    (Default|SetupLobbyMenu _aspaper_controller))
  (for _array_element_2 (Variables|Default|GetAllControllers)
    (bind _aspaper_controller_2 (Utilities|Casting|CastToPaperController _array_element_2))
    (Default|SaveUpdatedPlayerStats _aspaper_controller_2)
    (Utilities|Array|Add (Variables|Default|GetConnectedPlayers) (Variables|/Game/Blueprints/Characters/PaperController.PaperController_C|GetCharacterInformation _aspaper_controller_2)))
  (for _array_element_3 (Variables|Default|GetAllControllers)
    (bind _aspaper_controller_3 (Utilities|Casting|CastToPaperController _array_element_3))
    (Default|AddPlayerInformation _aspaper_controller_3 (Variables|Default|GetConnectedPlayers))))

(event Custom|AreAllPlayersFinished?
  (params (PlayerController :type Player%20Controller%20Object%20Reference) (bEnteredEndZone? :type Boolean))
  (bind _finishedplayers (Variables|Default|GetFinishedPlayers))
  (if (and (not (Utilities|Array|ContainsItem (Variables|Default|GetFinishedPlayers) PlayerController)) bEnteredEndZone?)
    (bind _returnvalue (Utilities|Array|Add _finishedplayers PlayerController))
    (if (== _returnvalue (Utilities|Array|LastIndex (Variables|Default|GetAllControllers)))
      _
      (else
        _))
    (CallFunction|GameIsFinished)
    (else
      (Utilities|Array|RemoveItem _finishedplayers PlayerController))))

(event Custom|PlayerRespawn
  (params (Controller :type Paper%20Controller%20Object%20Reference) (Player :type Paper%202D%20Character%20Object%20Reference))
  (Utilities|Respawn Controller Player))

(event Custom|AwardXPToAllPlayers
  (params (IncomingXP :type Float%20%28single-precision%29))
  (for _array_element (Variables|Default|GetAllControllers)
    (bind _aspaper_controller (Utilities|Casting|CastToPaperController _array_element))
    (Default|OwningClientAwardXP _aspaper_controller IncomingXP)))

(event EventPostLogin
  (params (NewPlayer :type Player%20Controller%20Object%20Reference))
  (Utilities|FlowControl|Delay 0.2)
  (Utilities|Array|Add (Variables|Default|GetAllControllers) NewPlayer)
  (bind _aspaper_controller (Utilities|Casting|CastToPaperController NewPlayer))
  (CallFunction|CreatePawn _aspaper_controller NewPlayer)
  (Default|CreateLoadingScreen _aspaper_controller)
  (Utilities|FlowControl|Delay 5.0)
  (Default|InitalSetup _aspaper_controller)
  (CallFunction|EveryoneUpdates))

(event EventAddXP
  (params (IncomingXP :type Float%20%28single-precision%29))
  (CallFunction|MulticastAwardXP IncomingXP))

(fn ConstructionScript)

(fn DamageAnimation
  (params (Paper2D%20Character :type Paper%202D%20Character%20Object%20Reference))
  (Camera|PlayWorldCameraShake "/Game/Blueprints/Camera/BP_CameraShake.BP_CameraShake_C" "0, 0, 0" 3e+03 5e+02 5.0)
  (return false))

(fn TimerDown
  (Utilities|Casting|CastToPaper2D_Character (Game|GetPlayerCharacter 0))
  (bind _returnvalue (UserInterface|CreateWidget "/Game/Widgets/WBP_CountDown.WBP_CountDown_C"))
  (bind _returnvalue_2 (UserInterface|Animation|PlayAnimation _returnvalue (Variables|Default|GetCountdown) 0.0 1 "Forward" 1.0 false))
  (return _returnvalue_2))

(fn CreatePawn
  (params (PaperController :type Paper%20Controller%20Object%20Reference) (PlayerController :type Player%20Controller%20Object%20Reference))
  (bind _spawnpoint (Variables|/Game/Blueprints/Characters/PaperController.PaperController_C|GetSpawnPoint PaperController))
  (bind _returnvalue (Class|GameModeBase|FindPlayerStart PaperController _spawnpoint))
  (bind _returnvalue_2 (Game|SpawnActorfromClass "/Game/Blueprints/Characters/Paper2D_Character.Paper2D_Character_C" (Math|Transform|MakeTransform (Transformation|GetActorLocation _returnvalue) (Transformation|GetActorRotation _returnvalue) "1,1,1") "Undefined" PlayerController 0))
  (Pawn|Possess PlayerController _returnvalue_2)
  (return))