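; A level room Blueprint for the ProGen level set, with doors that open while the 2D player character stands near them.
; Two trigger boxes each control a fixed group of door tiles: Box12 handles tiles 1 and 5, Box34 handles tiles 2, 3 and 4.
; Overlap by a Paper2D_Character hides those tiles and disables their collision, and ending the overlap restores both.
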(event OnComponentBeginOverlap(Box12)
  (params (OverlappedComponent :type Primitive%20Component%20Object%20Reference) (OtherActor :type Actor%20Object%20Reference) (OtherComp :type Primitive%20Component%20Object%20Reference) (OtherBodyIndex :type Integer) (bFromSweep :type Boolean) (SweepResult :type Hit%20Result%20Structure%20%28by%20ref%29))
  (bind _doortile1 (Variables|Default|GetDoorTile1))
  (bind _doortile5 (Variables|Default|GetDoorTile5))
  (Utilities|Casting|CastToPaper2D_Character OtherActor)
  (Rendering|SetVisibility _doortile1 false false)
  (Collision|SetCollisionEnabled _doortile1 "NoCollision")
  (Rendering|SetVisibility _doortile5 false false)
  (Collision|SetCollisionEnabled _doortile5 "NoCollision"))

(event OnComponentEndOverlap(Box12)
  (params (OverlappedComponent :type Primitive%20Component%20Object%20Reference) (OtherActor :type Actor%20Object%20Reference) (OtherComp :type Primitive%20Component%20Object%20Reference) (OtherBodyIndex :type Integer))
  (bind _doortile1 (Variables|Default|GetDoorTile1))
  (bind _doortile5 (Variables|Default|GetDoorTile5))
  (Utilities|Casting|CastToPaper2D_Character OtherActor)
  (Rendering|SetVisibility _doortile1 true false)
  (Collision|SetCollisionEnabled _doortile1 "QueryAndPhysics")
  (Rendering|SetVisibility _doortile5 true false)
  (Collision|SetCollisionEnabled _doortile5 "QueryAndPhysics"))

(event OnComponentBeginOverlap(Box34)
  (params (OverlappedComponent :type Primitive%20Component%20Object%20Reference) (OtherActor :type Actor%20Object%20Reference) (OtherComp :type Primitive%20Component%20Object%20Reference) (OtherBodyIndex :type Integer) (bFromSweep :type Boolean) (SweepResult :type Hit%20Result%20Structure%20%28by%20ref%29))
  (bind _doortile3 (Variables|Default|GetDoorTile3))
  (bind _doortile4 (Variables|Default|GetDoorTile4))
  (bind _doortile2 (Variables|Default|GetDoorTile2))
  (Utilities|Casting|CastToPaper2D_Character OtherActor)
  (Rendering|SetVisibility _doortile2 false false)
  (Collision|SetCollisionEnabled _doortile2 "NoCollision")
  (Rendering|SetVisibility _doortile4 false false)
  (Collision|SetCollisionEnabled _doortile4 "NoCollision")
  (Rendering|SetVisibility _doortile3 false false)
  (Collision|SetCollisionEnabled _doortile3 "NoCollision"))

(event OnComponentEndOverlap(Box34)
  (params (OverlappedComponent :type Primitive%20Component%20Object%20Reference) (OtherActor :type Actor%20Object%20Reference) (OtherComp :type Primitive%20Component%20Object%20Reference) (OtherBodyIndex :type Integer))
  (bind _doortile3 (Variables|Default|GetDoorTile3))
  (bind _doortile4 (Variables|Default|GetDoorTile4))
  (bind _doortile2 (Variables|Default|GetDoorTile2))
  (Utilities|Casting|CastToPaper2D_Character OtherActor)
  (Rendering|SetVisibility _doortile2 true false)
  (Collision|SetCollisionEnabled _doortile2 "QueryAndPhysics")
  (Rendering|SetVisibility _doortile4 true false)
  (Collision|SetCollisionEnabled _doortile4 "QueryAndPhysics")
  (Rendering|SetVisibility _doortile3 true false)
  (Collision|SetCollisionEnabled _doortile3 "QueryAndPhysics"))

(event EventBeginPlay
  (|CallParentFunction) ; This node is disabled and will not be called.\nDrag off pins to build functionality.
)

(event Collision|EventActorBeginOverlap
  (params (OtherActor :type Actor%20Object%20Reference))
  (|CallParentFunction OtherActor) ; This node is disabled and will not be called.\nDrag off pins to build functionality.
)

(event EventTick
  (params (DeltaSeconds :type Float%20%28single-precision%29))
  (|CallParentFunction DeltaSeconds) ; This node is disabled and will not be called.\nDrag off pins to build functionality.
)

(fn ConstructionScript
  (|CallParentFunction))