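; Large four-entry level room from the ProGenV6 assets, with doorways on the south, west, north and east sides.
; Each side has a box trigger paired with two door tiles.
; When a Paper2D_Character enters a box, that side's tiles are hidden and lose collision, then reappear solid when the character leaves.
; The construction script only calls its parent.
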(event OnComponentBeginOverlap(BoxS)
  (params (OverlappedComponent :type Primitive%20Component%20Object%20Reference) (OtherActor :type Actor%20Object%20Reference) (OtherComp :type Primitive%20Component%20Object%20Reference) (OtherBodyIndex :type Integer) (bFromSweep :type Boolean) (SweepResult :type Hit%20Result%20Structure%20%28by%20ref%29))
  (bind _doortile1 (Variables|Default|GetDoorTile1))
  (bind _doortile3 (Variables|Default|GetDoorTile3))
  (Utilities|Casting|CastToPaper2D_Character OtherActor)
  (Rendering|SetVisibility _doortile1 false false)
  (Collision|SetCollisionEnabled _doortile1 "NoCollision")
  (Rendering|SetVisibility _doortile3 false false)
  (Collision|SetCollisionEnabled _doortile3 "NoCollision"))

(event OnComponentEndOverlap(BoxS)
  (params (OverlappedComponent :type Primitive%20Component%20Object%20Reference) (OtherActor :type Actor%20Object%20Reference) (OtherComp :type Primitive%20Component%20Object%20Reference) (OtherBodyIndex :type Integer))
  (bind _doortile1 (Variables|Default|GetDoorTile1))
  (bind _doortile3 (Variables|Default|GetDoorTile3))
  (Utilities|Casting|CastToPaper2D_Character OtherActor)
  (Rendering|SetVisibility _doortile1 true false)
  (Collision|SetCollisionEnabled _doortile1 "QueryAndPhysics")
  (Rendering|SetVisibility _doortile3 true false)
  (Collision|SetCollisionEnabled _doortile3 "QueryAndPhysics"))

(event OnComponentBeginOverlap(BoxW)
  (params (OverlappedComponent :type Primitive%20Component%20Object%20Reference) (OtherActor :type Actor%20Object%20Reference) (OtherComp :type Primitive%20Component%20Object%20Reference) (OtherBodyIndex :type Integer) (bFromSweep :type Boolean) (SweepResult :type Hit%20Result%20Structure%20%28by%20ref%29))
  (bind _doortile4 (Variables|Default|GetDoorTile4))
  (bind _doortile2 (Variables|Default|GetDoorTile2))
  (Utilities|Casting|CastToPaper2D_Character OtherActor)
  (Rendering|SetVisibility _doortile4 false false)
  (Collision|SetCollisionEnabled _doortile4 "NoCollision")
  (Rendering|SetVisibility _doortile2 false false)
  (Collision|SetCollisionEnabled _doortile2 "NoCollision"))

(event OnComponentEndOverlap(BoxW)
  (params (OverlappedComponent :type Primitive%20Component%20Object%20Reference) (OtherActor :type Actor%20Object%20Reference) (OtherComp :type Primitive%20Component%20Object%20Reference) (OtherBodyIndex :type Integer))
  (bind _doortile4 (Variables|Default|GetDoorTile4))
  (bind _doortile2 (Variables|Default|GetDoorTile2))
  (Utilities|Casting|CastToPaper2D_Character OtherActor)
  (Rendering|SetVisibility _doortile4 true false)
  (Collision|SetCollisionEnabled _doortile4 "QueryAndPhysics")
  (Rendering|SetVisibility _doortile2 true false)
  (Collision|SetCollisionEnabled _doortile2 "QueryAndPhysics"))

(event OnComponentEndOverlap(BoxN)
  (params (OverlappedComponent :type Primitive%20Component%20Object%20Reference) (OtherActor :type Actor%20Object%20Reference) (OtherComp :type Primitive%20Component%20Object%20Reference) (OtherBodyIndex :type Integer))
  (bind _doortile5 (Variables|Default|GetDoorTile5))
  (bind _doortile6 (Variables|Default|GetDoorTile6))
  (Utilities|Casting|CastToPaper2D_Character OtherActor)
  (Rendering|SetVisibility _doortile5 true false)
  (Collision|SetCollisionEnabled _doortile5 "QueryAndPhysics")
  (Rendering|SetVisibility _doortile6 true false)
  (Collision|SetCollisionEnabled _doortile6 "QueryAndPhysics"))

(event OnComponentBeginOverlap(BoxE)
  (params (OverlappedComponent :type Primitive%20Component%20Object%20Reference) (OtherActor :type Actor%20Object%20Reference) (OtherComp :type Primitive%20Component%20Object%20Reference) (OtherBodyIndex :type Integer) (bFromSweep :type Boolean) (SweepResult :type Hit%20Result%20Structure%20%28by%20ref%29))
  (bind _doortile7 (Variables|Default|GetDoorTile7))
  (bind _doortile8 (Variables|Default|GetDoorTile8))
  (Utilities|Casting|CastToPaper2D_Character OtherActor)
  (Rendering|SetVisibility _doortile7 false false)
  (Collision|SetCollisionEnabled _doortile7 "NoCollision")
  (Rendering|SetVisibility _doortile8 false false)
  (Collision|SetCollisionEnabled _doortile8 "NoCollision"))

(event OnComponentEndOverlap(BoxE)
  (params (OverlappedComponent :type Primitive%20Component%20Object%20Reference) (OtherActor :type Actor%20Object%20Reference) (OtherComp :type Primitive%20Component%20Object%20Reference) (OtherBodyIndex :type Integer))
  (bind _doortile7 (Variables|Default|GetDoorTile7))
  (bind _doortile8 (Variables|Default|GetDoorTile8))
  (Utilities|Casting|CastToPaper2D_Character OtherActor)
  (Rendering|SetVisibility _doortile7 true false)
  (Collision|SetCollisionEnabled _doortile7 "QueryAndPhysics")
  (Rendering|SetVisibility _doortile8 true false)
  (Collision|SetCollisionEnabled _doortile8 "QueryAndPhysics"))

(event OnComponentBeginOverlap(BoxN)
  (params (OverlappedComponent :type Primitive%20Component%20Object%20Reference) (OtherActor :type Actor%20Object%20Reference) (OtherComp :type Primitive%20Component%20Object%20Reference) (OtherBodyIndex :type Integer) (bFromSweep :type Boolean) (SweepResult :type Hit%20Result%20Structure%20%28by%20ref%29))
  (bind _doortile5 (Variables|Default|GetDoorTile5))
  (bind _doortile6 (Variables|Default|GetDoorTile6))
  (Utilities|Casting|CastToPaper2D_Character OtherActor)
  (Rendering|SetVisibility _doortile5 false false)
  (Collision|SetCollisionEnabled _doortile5 "NoCollision")
  (Rendering|SetVisibility _doortile6 false false)
  (Collision|SetCollisionEnabled _doortile6 "NoCollision"))

(event EventBeginPlay
  (|CallParentFunction) ; This node is disabled and will not be called.\nDrag off pins to build functionality.
)

(event Collision|EventActorBeginOverlap
  (params (OtherActor :type Actor%20Object%20Reference))
  (|CallParentFunction OtherActor) ; This node is disabled and will not be called.\nDrag off pins to build functionality.
)

(event EventTick
  (params (DeltaSeconds :type Float%20%28single-precision%29))
  (|CallParentFunction DeltaSeconds) ; This node is disabled and will not be called.\nDrag off pins to build functionality.
)

(fn ConstructionScript
  (|CallParentFunction))