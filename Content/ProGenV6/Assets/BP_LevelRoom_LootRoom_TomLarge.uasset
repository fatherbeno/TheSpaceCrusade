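; Loot room level piece, named as a large variant for procedural generation, with a proximity-triggered door.
; When a Paper2D_Character enters the Box trigger, both door tiles are hidden and their collision is disabled.
; When the character leaves, the tiles reappear with query and physics collision restored.
; The construction script only calls its parent, and the default BeginPlay, overlap and Tick events are disabled.
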(event OnComponentBeginOverlap(Box)
  (params (OverlappedComponent :type Primitive%20Component%20Object%20Reference) (OtherActor :type Actor%20Object%20Reference) (OtherComp :type Primitive%20Component%20Object%20Reference) (OtherBodyIndex :type Integer) (bFromSweep :type Boolean) (SweepResult :type Hit%20Result%20Structure%20%28by%20ref%29))
  (bind _doortile1 (Variables|Default|GetDoorTile1))
  (bind _doortile2 (Variables|Default|GetDoorTile2))
  (Utilities|Casting|CastToPaper2D_Character OtherActor)
  (Rendering|SetVisibility _doortile1 false false)
  (Collision|SetCollisionEnabled _doortile1 "NoCollision")
  (Rendering|SetVisibility _doortile2 false false)
  (Collision|SetCollisionEnabled _doortile2 "NoCollision"))

(event OnComponentEndOverlap(Box)
  (params (OverlappedComponent :type Primitive%20Component%20Object%20Reference) (OtherActor :type Actor%20Object%20Reference) (OtherComp :type Primitive%20Component%20Object%20Reference) (OtherBodyIndex :type Integer))
  (bind _doortile1 (Variables|Default|GetDoorTile1))
  (bind _doortile2 (Variables|Default|GetDoorTile2))
  (Utilities|Casting|CastToPaper2D_Character OtherActor)
  (Rendering|SetVisibility _doortile1 true false)
  (Collision|SetCollisionEnabled _doortile1 "QueryAndPhysics")
  (Rendering|SetVisibility _doortile2 true false)
  (Collision|SetCollisionEnabled _doortile2 "QueryAndPhysics"))

(event EventBeginPlay
  (|CallParentFunction) ; This node is disabled and will not be called.\nDrag off pins to build functionality.
)

(event Collision|EventActorBeginOverlap
  (params (OtherActor :type Actor%20Object%20Reference))
  (|CallParentFunction OtherActor) ; This node is disabled and will not be called.\nDrag off pins to build functionality.
)

(event EventTick
  (params (DeltaSeconds :type Float%20%28single-precision%29))
  (|CallParentFunction DeltaSeconds) ; This node is disabled and will not be called.\nDrag off pins to build functionality.
)

(fn ConstructionScript
  (|CallParentFunction))